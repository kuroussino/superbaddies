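; BP_DefaultCamera is a player-controlled camera pawn with smoothed zoom, planar movement and yaw rotation.
; On BeginPlay it registers an Enhanced Input mapping context through BP_DefaultPC, then seeds its targets from the current spring arm length and actor transform.
; Input actions adjust those targets, clamping zoom range and moving relative to the actor's facing.
; Tick interpolates arm length, location and rotation toward the targets, each at its own speed.
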(event Input|EnhancedActionEvents|EnhancedInputActionIA_ZoomCamera
  (params (ActionValue :type Float%20%28double-precision%29) (ElapsedSeconds :type Float%20%28double-precision%29) (TriggeredSeconds :type Float%20%28double-precision%29) (InputAction :type Input%20Action%20Object%20Reference :default "/Game/Superbaddies/Core/Input/Actions/IA_ZoomCamera.IA_ZoomCamera"))
  ;[1 1 1] IMC
  (Variables|Default|SetzoomSmoothTarget (Math|Float|Clamp(Float) (+ (* ActionValue (Variables|Default|GetzoomMultiplier)) (Variables|Default|GetzoomSmoothTarget)) (Variables|Default|GetzoomMin) (Variables|Default|GetzoomMax))))

(event Input|EnhancedActionEvents|EnhancedInputActionIA_MoveCamera
  (params (ActionValue :type Vector%202D%20Structure) (ElapsedSeconds :type Float%20%28double-precision%29) (TriggeredSeconds :type Float%20%28double-precision%29) (InputAction :type Input%20Action%20Object%20Reference :default "/Game/Superbaddies/Core/Input/Actions/IA_MoveCamera.IA_MoveCamera"))
  (bind (_x _y) (Math|Vector2D|BreakVector2D ActionValue))
  ;[1 1 1] IMC
  (Variables|Default|SetmoveSmoothTarget (+ (Variables|Default|GetmoveSmoothTarget) (* (Math|Vector|ClampVectorSize (+ (* (Transformation|GetActorForwardVector) _y) (* (Transformation|GetActorRightVector) _x)) 0.0 1.0) (Variables|Default|GetmoveMultiplier)))))

(event Input|EnhancedActionEvents|EnhancedInputActionIA_RotateCamera
  (params (ActionValue :type Float%20%28double-precision%29) (ElapsedSeconds :type Float%20%28double-precision%29) (TriggeredSeconds :type Float%20%28double-precision%29) (InputAction :type Input%20Action%20Object%20Reference :default "/Game/Superbaddies/Core/Input/Actions/IA_RotateCamera.IA_RotateCamera"))
  ;[1 1 1] IMC
  (Variables|Default|SetrotateSmoothTarget (Math|Rotator|CombineRotators (Variables|Default|GetrotateSmoothTarget) (Math|Rotator|MakeRotator 0.0 0.0 (* ActionValue (Variables|Default|GetrotateMultiplier))))))

(event EventBeginPlay
  (Utilities|InitializeIMC
    (:out
      (Variables|Default|SetzoomSmoothTarget (Variables|/Script/Engine.SpringArmComponent|GetTargetArmLength (Variables|Default|GetSpringArm)))
      (Variables|Default|SetmoveSmoothTarget (Transformation|GetActorLocation))
      (Variables|Default|SetrotateSmoothTarget (Transformation|GetActorRotation)))))

(event EventTick
  (params (DeltaSeconds :type Float%20%28single-precision%29))
  (Utilities|FlowControl|Sequence
    (:then_0
      (if (!= (Variables|Default|GetzoomSmoothTarget) (Variables|/Script/Engine.SpringArmComponent|GetTargetArmLength (Variables|Default|GetSpringArm)))
        (Variables|/Script/Engine.SpringArmComponent|SetTargetArmLength (Variables|Default|GetSpringArm) (Math|Interpolation|FInterpTo (Variables|/Script/Engine.SpringArmComponent|GetTargetArmLength (Variables|Default|GetSpringArm)) (Variables|Default|GetzoomSmoothTarget) (Utilities|Time|GetWorldDeltaSeconds) (Variables|Default|GetzoomSmoothSpeed)))))
    (:then_1
      (if (Utilities|Operators|NotEqual(!=) (Variables|Default|GetmoveSmoothTarget) (Transformation|GetActorLocation) 0.0)
        (Transformation|SetActorLocation (Math|Interpolation|VInterpTo (Transformation|GetActorLocation) (Variables|Default|GetmoveSmoothTarget) (Utilities|Time|GetWorldDeltaSeconds) (Variables|Default|GetmoveSmoothSpeed)) false false)))
    (:then_2
      (if (Utilities|Operators|NotEqual(!=) (Variables|Default|GetrotateSmoothTarget) (Transformation|GetActorRotation) 0.0)
        (Transformation|SetActorRotation (Math|Interpolation|RInterpTo (Transformation|GetActorRotation) (Variables|Default|GetrotateSmoothTarget) (Utilities|Time|GetWorldDeltaSeconds) (Variables|Default|GetrotateSmoothSpeed)))))))

(fn ConstructionScript)